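; BP_MainLightController scales down directional-light shadows by enemy count in the Apparatus shoot-em-up, apparently as a performance measure.
; Each Tick it samples the ShadowByEnemyCount curve with the current EnemiesCount to set the owner's shadow amount and SecondaryLight's intensity.
; When the curve nears zero, it disables shadow casting and destroys SecondaryLight, with no path to restore either.
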(event EventBeginPlay)

(event EventTick
  (params (DeltaSeconds :type Float%20%28single-precision%29))
  (bind _returnvalue (Components|GetOwner))
  (bind _returnvalue_2 (Class|EnemySpawner|GetInstance))
  (bind _shadow_by_enemy_count (Variables|Default|GetShadow%20by%20Enemy%20Count))
  (bind _returnvalue_3 (Actor|GetComponentbyClass _returnvalue "/Script/Engine.DirectionalLightComponent"))
  (bind _enemiescount (Variables|/Script/ApparatusShootEmUp.EnemySpawner|GetEnemiesCount _returnvalue_2))
  (bind _returnvalue_4 (Math|Conversions|ToFloat(Integer) _enemiescount))
  (bind _returnvalue_5 (Math|Curves|GetFloatValue _shadow_by_enemy_count _returnvalue_4))
  (if (<= _returnvalue_5 0.001)
    (Rendering|Components|Light|SetCastShadows _returnvalue_3 false)
    (Actor|DestroyActor (Variables|Default|GetSecondary%20Light))
    (else
      (Class|DirectionalLightComponent|SetShadowAmount _returnvalue_3 _returnvalue_5)
      (Rendering|Components|Light|SetIntensity (Variables|/Script/Engine.Light|GetLightComponent (Variables|Default|GetSecondary%20Light)) (* _returnvalue_5 3.0)))))